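; SH_BP_Vector is a lecture Blueprint that demonstrates moving an actor with vector math.
; On BeginPlay it offsets its location a fixed distance along the normalized forward vector derived from its own rotation, without sweeping.
; Two disconnected variants remain in the graph: a fixed world X offset and an offset along a fixed yaw direction.
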(event EventBeginPlay
  (Transformation|SetActorLocation (+ (Transformation|GetActorLocation) (* (Math|Vector|Normalize (Math|Vector|GetForwardVector (Transformation|GetActorRotation))) 2e+02)) false false))

(fn ConstructionScript)